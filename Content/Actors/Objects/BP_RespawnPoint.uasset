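; BP_RespawnPoint is a checkpoint trigger that updates where the player character respawns.
; When the player's character overlaps the box collider, it stores RespawnLocation as that character's CurrentRespawnPoint and briefly shows the respawn text on its GUI.
; The construction script sizes and positions the collider from the BoxScale and BoxColliderLocation variables.
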(event OnComponentBeginOverlap(BoxCollider)
  (params (OverlappedComponent :type Primitive%20Component%20Object%20Reference) (OtherActor :type Actor%20Object%20Reference) (OtherComp :type Primitive%20Component%20Object%20Reference) (OtherBodyIndex :type Integer) (bFromSweep :type Boolean) (SweepResult :type Hit%20Result%20Structure%20%28by%20ref%29))
  (bind _myplayercharacter (CallFunction|GetMyPlayerCharacter))
  (bind _myplayercharacter_2 (CallFunction|GetMyPlayerCharacter))
  (bind _gui (Variables|/Game/Actors/MyPlayerCharacter/BP_MyPlayerCharacter.BP_MyPlayerCharacter_C|GetGUI _myplayercharacter_2))
  (bind _respawntext (Variables|/Game/Core/UI/WBP_GUI.WBP_GUI_C|GetRespawnText _gui))
  (if (== OtherActor _myplayercharacter)
    (Variables|/Game/Actors/MyPlayerCharacter/BP_MyPlayerCharacter.BP_MyPlayerCharacter_C|SetCurrentRespawnPoint _myplayercharacter (Variables|Default|GetRespawnLocation))
    (Widget|SetVisibility _respawntext "SelfHitTestInvisible")
    (Utilities|FlowControl|Delay 1.0)
    (Widget|SetVisibility _respawntext "Hidden")))

(fn ConstructionScript
  (bind _boxcollider (Variables|Default|GetBoxCollider))
  (Transformation|SetWorldScale3D _boxcollider (Variables|Default|GetBoxScale))
  (Transformation|SetRelativeLocation _boxcollider (Variables|Default|GetBoxColliderLocation) false false))