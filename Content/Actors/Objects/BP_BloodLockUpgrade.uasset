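; Blood lock upgrade object that rewards the player with an upgrade once every enemy in its Enemies list is destroyed.
; On BeginPlay it binds to each enemy's OnDestroyed event and stores the enemy count, which drops with each death.
; At zero it opens the upgrade menu through the player controller's UI root and clears the player character's in-combat flag.
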(event Custom|OnDeath
  (params (DestroyedActor :type Actor%20Object%20Reference))
  (bind _result (Math|Integer|DecrementInt (Variables|Default|GetRemaining))
    (:%20%20
      (if (== _result 0)
        (CallFunction|Completed)))))

(event Custom|Completed
  (Default|OpenUpgradeMenu (Variables|/Game/Core/PC_MyPlayerController.PC_MyPlayerController_C|GetUIRoot (CallFunction|GetMyPlayerController)))
  (Variables|/Game/Actors/MyPlayerCharacter/BP_MyPlayerCharacter.BP_MyPlayerCharacter_C|SetIsInCombat (CallFunction|GetMyPlayerCharacter) false))

(event EventBeginPlay
  (for _array_element (Variables|Default|GetEnemies)
    (Game|BindEventtoOnDestroyed _array_element (delegate Custom|OnDeath))
    (Variables|Default|SetRemaining (Utilities|Array|Length (Variables|Default|GetEnemies)))))

(fn ConstructionScript)