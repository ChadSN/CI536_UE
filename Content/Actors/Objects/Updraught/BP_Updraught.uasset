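; Updraught fan actor that pushes the player character along its area of effect while they overlap its box.
; The construction script positions and sizes the box between the AoE start and end points.
; Each tick applies a velocity-change impulse along character up plus fan direction, scaled by Force and a distance-sampled strength curve.
; A second distance curve dampens falling by limiting downward Z velocity.
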(event OnComponentBeginOverlap(BoxCollision)
  (params (OverlappedComponent :type Primitive%20Component%20Object%20Reference) (OtherActor :type Actor%20Object%20Reference) (OtherComp :type Primitive%20Component%20Object%20Reference) (OtherBodyIndex :type Integer) (bFromSweep :type Boolean) (SweepResult :type Hit%20Result%20Structure%20%28by%20ref%29))
  (bind _returnvalue (Game|GetPlayerCharacter 0))
  (if (== OtherActor _returnvalue)
    (Variables|Default|SetCharacter _returnvalue)))

(event OnComponentEndOverlap(BoxCollision)
  (params (OverlappedComponent :type Primitive%20Component%20Object%20Reference) (OtherActor :type Actor%20Object%20Reference) (OtherComp :type Primitive%20Component%20Object%20Reference) (OtherBodyIndex :type Integer))
  (bind _character (Variables|Default|GetCharacter)
    (:then
      (if (== _character OtherActor)
        (Variables|Default|SetCharacter 0)))
    (:else)))

(event EventTick
  (params (DeltaSeconds :type Float%20%28single-precision%29))
  (bind _character (Variables|Default|GetCharacter))
  (bind _returnvalue (Transformation|GetVelocity _character))
  ;[0 0 0] Is Character Valid?
  (bind _character_2 (Variables|Default|GetCharacter)
    (:then
      ;[0 0 0] Add (BoxCollision Up Vector * Force Multiplier) to Impulse
      (Physics|AddImpulse (Variables|/Script/Engine.Character|GetCharacterMovement _character_2) (* (+ (Transformation|GetActorUpVector (Variables|Default|GetCharacter)) (Math|Vector|Normalize (- (Transformation|GetWorldLocation (Variables|Default|GetFan_AoE_End)) (Transformation|GetWorldLocation (Variables|Default|GetFan_AoE_Start))))) (* (Math|Curves|GetFloatValue (Variables|Default|GetC_FanStrength) (Math|Float|Clamp(Float) (Utilities|Operators|Divide (Math|Vector|Distance(Vector) (Transformation|GetActorLocation _character_2) (Transformation|GetWorldLocation (Variables|Default|GetFan_AoE_Start))) (Math|Vector|Distance(Vector) (Variables|Default|GetAoE_Start) (Variables|Default|GetAoE_End)) 2.0))) (Variables|Default|GetForce))) true)
      ;[0 0 0] Dampen Z velocity with inverse normalised distance curve using a clamp on Z velocity
      (Variables|/Script/Engine.MovementComponent|SetVelocity (Variables|/Script/Engine.Character|GetCharacterMovement (Variables|Default|GetCharacter)) (Math|Vector|MakeVector (.x _returnvalue) (.y _returnvalue) (Math|Float|Clamp(Float) (.z _returnvalue) (* (Math|Curves|GetFloatValue (Variables|Default|GetC_FanDampening) (Math|Float|Clamp(Float) (Utilities|Operators|Divide (Math|Vector|Distance(Vector) (Transformation|GetActorLocation _character_2) (Transformation|GetWorldLocation (Variables|Default|GetFan_AoE_Start))) (Math|Vector|Distance(Vector) (Variables|Default|GetAoE_Start) (Variables|Default|GetAoE_End)) 2.0))) -4e+03) 4e+03))))
    (:else)))

(fn ConstructionScript
  (Variables|Default|SetAoE_Start (Variables|/Script/Engine.SceneComponent|GetRelativeLocation (Variables|Default|GetFan_AoE_Start)))
  (Transformation|SetRelativeLocation (Variables|Default|GetFan_AoE_End) (Variables|Default|GetAoE_End) false false)
  (Components|Box|SetBoxExtent (Variables|Default|GetBoxCollision) (Math|Vector|MakeVector 1e+02 1e+02 (/ (Math|Vector|Distance(Vector) (Variables|Default|GetAoE_Start) (Variables|Default|GetAoE_End)) 2.0)) true)
  (Transformation|SetRelativeLocation (Variables|Default|GetBoxCollision) (/ (+ (Variables|Default|GetAoE_Start) (Variables|Default|GetAoE_End)) 2.0) false false))