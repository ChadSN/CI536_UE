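; BP_CombatRoom is a combat room actor that tracks a set of enemies and opens the upgrade menu once all are destroyed.
; On BeginPlay it binds each entry in Enemies to OnDestroyed and counts down a Remaining counter as they die.
; A Box overlap toggles the player character's IsInCombat flag on enter and exit, and clearing the room also resets it to false.
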(event OnComponentBeginOverlap(Box)
  (params (OverlappedComponent :type Primitive%20Component%20Object%20Reference) (OtherActor :type Actor%20Object%20Reference) (OtherComp :type Primitive%20Component%20Object%20Reference) (OtherBodyIndex :type Integer) (bFromSweep :type Boolean) (SweepResult :type Hit%20Result%20Structure%20%28by%20ref%29))
  (bind _asbp_my_player_character (Utilities|Casting|CastToBP_MyPlayerCharacter OtherActor))
  (Variables|/Game/Actors/MyPlayerCharacter/BP_MyPlayerCharacter.BP_MyPlayerCharacter_C|SetIsInCombat _asbp_my_player_character true))

(event OnComponentEndOverlap(Box)
  (params (OverlappedComponent :type Primitive%20Component%20Object%20Reference) (OtherActor :type Actor%20Object%20Reference) (OtherComp :type Primitive%20Component%20Object%20Reference) (OtherBodyIndex :type Integer))
  (bind _asbp_my_player_character (Utilities|Casting|CastToBP_MyPlayerCharacter OtherActor))
  (Variables|/Game/Actors/MyPlayerCharacter/BP_MyPlayerCharacter.BP_MyPlayerCharacter_C|SetIsInCombat _asbp_my_player_character false))

(event Custom|OnDeath
  (params (DestroyedActor :type Actor%20Object%20Reference))
  (bind _result (Math|Integer|DecrementInt (Variables|Default|GetRemaining))
    (:%20%20
      (if (== _result 0)
        (CallFunction|Completed)))))

(event Custom|Completed
  (Default|OpenUpgradeMenu (Variables|/Game/Core/PC_MyPlayerController.PC_MyPlayerController_C|GetUIRoot (CallFunction|GetMyPlayerController)))
  (Variables|/Game/Actors/MyPlayerCharacter/BP_MyPlayerCharacter.BP_MyPlayerCharacter_C|SetIsInCombat (CallFunction|GetMyPlayerCharacter) false))

(event EventBeginPlay
  (for _array_element (Variables|Default|GetEnemies)
    (Game|BindEventtoOnDestroyed _array_element (delegate Custom|OnDeath))
    (Variables|Default|SetRemaining (Utilities|Array|Length (Variables|Default|GetEnemies)))))

(fn ConstructionScript)