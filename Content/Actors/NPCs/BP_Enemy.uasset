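; Base enemy character that chases the player with AI MoveTo and calls an overridable AttackPlayer on arrival, retrying when the move fails.
; While engaged it turns toward the player each Tick.
; When ShouldAttackTrace is set, a socket sphere trace damages and knocks back a non-invulnerable player.
; Incoming damage goes through the health component, causing knockback and a hit montage, or death with player stamina recovery, montage and destruction.
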(event Custom|ChaseCharacter
  ;[0.15 0.15 0.15 0.5] Chase Character
  (if (not (Variables|Default|GetIsDead))
    (AI|AIMoveTo self "0, 0, 0" (CallFunction|GetMyPlayerCharacter) 125.0 false
      (:then
        (Variables|Default|SetIsEngaged true))
      (:OnSuccess
        (CallFunction|AttackPlayer))
      (:OnFail
        (Utilities|FlowControl|Delay 1.0)
        (CallFunction|ChaseCharacter)
        (Variables|Default|SetIsEngaged false)))))

(event Custom|AttackPlayer
  ;[0.15 0.15 0.15 0.5] Overridable Event
)

(event Custom|Death
  (bind _mesh (Variables|Character|GetMesh))
  ;[0.15 0.15 0.15 0.5] Death
  (Variables|Default|SetIsEngaged false)
  (Default|StartStaminaRecovery (CallFunction|GetMyPlayerCharacter))
  (Components|Movement|StopMovementImmediately (Variables|Character|GetCharacterMovement))
  (Variables|Default|SetIsDead true)
  (Audio|Components|Audio|Stop _mesh)
  (Animation|Montage|PlayMontage _mesh (Variables|Default|GetDeathMontage)
    (:OnCompleted
      _)
    (:OnInterrupted
      (Utilities|FlowControl|Delay 1.0)))
  (Actor|DestroyActor))

(event EventTick
  (params (DeltaSeconds :type Float%20%28single-precision%29))
  (bind _returnvalue (Game|GetPlayerCharacter 0))
  (bind _returnvalue_2 (Transformation|GetActorLocation))
  (bind _mesh (Variables|Character|GetMesh))
  (bind _attacklaunchforce (Variables|Default|GetAttackLaunchForce))
  (bind _in_socket_name (Variables|Default|GetIn%20Socket%20Name))
  (bind _returnvalue_3 (Transformation|GetSocketLocation _mesh _in_socket_name))
  (bind _returnvalue_4 (Transformation|GetActorLocation _returnvalue))
  (bind _returnvalue_5 (- _returnvalue_4 _returnvalue_2))
  (bind _returnvalue_6 (Math|Vector|Normalize _returnvalue_5))
  (bind _returnvalue_7 (* _returnvalue_6 _attacklaunchforce))
  (Utilities|FlowControl|Sequence
    (:then_0
      ;[0.15 0.15 0.15 0.5] Attack Trace
      (if (Variables|Default|GetShouldAttackTrace)
        (bind (_outhit _returnvalue_8) (Collision|SphereTraceForObjects _returnvalue_3 _returnvalue_3 2e+01 (Utilities|Array|MakeArray "ObjectTypeQuery3") false 0 "None"))
        (if _returnvalue_8
          (if (== (.HitActor (Collision|BreakHitResult _outhit)) _returnvalue)
            (if (not (Variables|/Game/Actors/MyPlayerCharacter/BP_MyPlayerCharacter.BP_MyPlayerCharacter_C|GetInvulnerable (CallFunction|GetMyPlayerCharacter)))
              (Game|Damage|ApplyDamage _returnvalue (Variables|Default|GetAttackDamage) 0 self)
              (Character|LaunchCharacter _returnvalue (Math|Vector|MakeVector (.x _returnvalue_7) (.y _returnvalue_7) 1.5e+02) false false))
            (Variables|Default|SetShouldAttackTrace false)))))
    (:then_1
      (if (Variables|Default|GetIsEngaged)
        (Transformation|SetActorRotation (Math|Rotator|MakeRotator 0.0 0.0 (.yaw (Class|KismetMathLibrary|RInterptoConstant (Transformation|GetActorRotation) (Math|Rotator|FindLookatRotation (Transformation|GetActorLocation) (Transformation|GetActorLocation (Game|GetPlayerCharacter 0))) (Utilities|Time|GetWorldDeltaSeconds) 1e+02))))))))

(event Game|Damage|EventAnyDamage
  (params (Damage :type Float%20%28single-precision%29) (DamageType :type Damage%20Type%20Object%20Reference) (InstigatedBy :type Controller%20Object%20Reference) (DamageCauser :type Actor%20Object%20Reference))
  (bind _returnvalue (Transformation|GetActorLocation DamageCauser))
  (bind _returnvalue_2 (Transformation|GetActorLocation))
  (bind _mesh (Variables|Character|GetMesh))
  (bind _returnvalue_3 (- _returnvalue_2 _returnvalue))
  (bind _returnvalue_4 (Math|Vector|Normalize _returnvalue_3))
  (bind _returnvalue_5 (* _returnvalue_4 7.5e+02))
  ;[0.15 0.15 0.15 0.5] Event Any Damage
  (bind _isdead (Default|ChangeHealth (Variables|Default|GetAC_HealthComponent) Damage))
  (if _isdead
    (CallFunction|Death)
    (else
      (Character|LaunchCharacter (Math|Vector|MakeVector (.x _returnvalue_5) (.y _returnvalue_5) 1.5e+02) false false)
      (Audio|Components|Audio|Stop _mesh)
      (bind _damagemontage (Variables|Default|GetDamageMontage)
        (:then
          (Animation|Montage|PlayMontage _mesh _damagemontage))
        (:else)))))

(fn ConstructionScript)