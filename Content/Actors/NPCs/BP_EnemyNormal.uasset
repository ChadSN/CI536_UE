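; Normal enemy NPC that wakes when the player enters its sphere collider, playing a get-up montage with attached sound before chasing.
; The overlap sets Engaged on the actor and its AnimBP, then fades the sound once the montage ends or is interrupted.
; The AttackPlayer override randomly plays one of two attack montages, skipped if either side is dead or it is stunned.
; Completed attacks resume the chase; interrupted ones first wait out the parry stun.
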(event OnComponentBeginOverlap(SphereCollider)
  (params (OverlappedComponent :type Primitive%20Component%20Object%20Reference) (OtherActor :type Actor%20Object%20Reference) (OtherComp :type Primitive%20Component%20Object%20Reference) (OtherBodyIndex :type Integer) (bFromSweep :type Boolean) (SweepResult :type Hit%20Result%20Structure%20%28by%20ref%29))
  ;[0.15 0.15 0.15 0.5] OnComponentBeginOverlap
  (if (not (Variables|Default|GetEngaged))
    (if (== OtherActor (Game|GetPlayerCharacter 0))
      (bind _asabp_enemy_normal (Utilities|Casting|CastToABP_EnemyNormal (Components|SkeletalMesh|GetAnimInstance (Variables|Character|GetMesh))))
      (Default|SetEngaged _asabp_enemy_normal)
      (Variables|Default|SetEngaged true)
      (Animation|Montage|PlayMontage (Variables|Character|GetMesh) "/Game/Actors/NPCs/Normal/Animations/AM_EnemyNormalGetUp.AM_EnemyNormalGetUp"
        (:then
          (bind _returnvalue (Audio|SpawnSoundAttached "/Game/Audio/NPCs/GetUp.GetUp" (Variables|Default|GetCapsuleComponent) "None" "0, 0, 0" "0, 0, 0" "KeepRelativeOffset" false 1.0 1.0 0.0 "/Game/Audio/SA_Default.SA_Default" 0))
          (Variables|Default|SetGetUpSound _returnvalue))
        (:OnCompleted
          (bind _getupsound (Variables|Default|GetGetUpSound :!label _label)
            (:then
              (Audio|Components|Audio|FadeOut _getupsound 0.5 0.0 "Linear" :!class /Script/Engine.AudioComponent))
            (:else
              _))
          (CallFunction|ChaseCharacter))
        (:OnInterrupted
          (goto _label))))))

(event EventAttackPlayer
  (bind _mesh (Variables|Character|GetMesh))
  ;[0.15 0.15 0.15 0.5] AttackPlayer Override
  (if (not (Math|Boolean|ORBoolean (Variables|Default|GetIsDead) (Variables|Default|GetIsStunned) (Variables|/Game/Actors/MyPlayerCharacter/BP_MyPlayerCharacter.BP_MyPlayerCharacter_C|GetIsDead (CallFunction|GetMyPlayerCharacter))))
    (if (Math|Random|RandomBool)
      (Animation|Montage|PlayMontage _mesh "/Game/Actors/NPCs/Normal/Animations/AM_Attack1.AM_Attack1"
        (:then
          (Variables|Default|SetIsAttacking true :!label _label))
        (:OnCompleted
          (CallFunction|ChaseCharacter :!label _label_2)
          (Variables|Default|SetIsAttacking false))
        (:OnInterrupted
          (Utilities|FlowControl|Delay (Variables|Default|GetParryStunDuration) :!label _label_3)
          (Variables|Default|SetIsStunned false)
          (goto _label_2)))
      (else
        (Animation|Montage|PlayMontage _mesh "/Game/Actors/NPCs/Normal/Animations/AM_Attack2.AM_Attack2"
          (:then
            (goto _label))
          (:OnCompleted
            (goto _label_2))
          (:OnInterrupted
            (goto _label_3)))))))

(fn ConstructionScript
  (|CallParentFunction))