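; Health component that tracks an actor's current health against a maximum.
; ChangeHealth subtracts the given value, clamps the result between zero and the maximum, and returns whether health is depleted.
; RestoreHealth refills to the maximum and sets the health bar in the player character's GUI to full; ChangeHealth leaves the bar untouched.
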(fn ChangeHealth
  (params (Value :type Float%20%28double-precision%29))
  (bind _output_get (Variables|Default|SetCurrentHealth (Math|Float|Clamp(Float) (- (Variables|Default|GetCurrentHealth) Value) 0.0 (Variables|Default|GetMaxHealth))))
  (return (<= _output_get 0.0)))

(fn RestoreHealth
  (Variables|Default|SetCurrentHealth (Variables|Default|GetMaxHealth))
  (Progress|SetPercent (Variables|/Game/Core/UI/WBP_GUI.WBP_GUI_C|GetHealthBar (Variables|/Game/Actors/MyPlayerCharacter/BP_MyPlayerCharacter.BP_MyPlayerCharacter_C|GetGUI (CallFunction|GetMyPlayerCharacter))) 1e+02))