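; Actor component that stores a stamina value and exposes functions to change, restore, deplete and query it.
; ChangeStamina subtracts the given amount, clamps the result between zero and MaxStamina, and reports whether stamina is depleted or full.
; Only RestoreStamina updates the HUD stamina bar, reached through the player controller's UI root; the other functions leave the UI untouched.
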(fn ChangeStamina
  (params (Value :type Float%20%28double-precision%29))
  (bind _output_get (Variables|Default|SetCurrentStamina (Math|Float|Clamp(Float) (- (Variables|Default|GetCurrentStamina) Value) 0.0 (Variables|Default|GetMaxStamina))))
  (return (<= _output_get 0.0) (>= _output_get (Variables|Default|GetMaxStamina))))

(fn RestoreStamina
  (Variables|Default|SetCurrentStamina (Variables|Default|GetMaxStamina))
  (Progress|SetPercent (Variables|/Game/Core/UI/WBP_GUI.WBP_GUI_C|GetStaminaBar (Variables|/Game/Core/UI/WBP_UIRoot.WBP_UIRoot_C|GetGUI (Variables|/Game/Core/PC_MyPlayerController.PC_MyPlayerController_C|GetUIRoot (CallFunction|GetMyPlayerController)))) 1e+02))

(fn DepleteStamina
  (Variables|Default|SetCurrentStamina 0.0))

(fn IsDepleted
  (return (<= (Variables|Default|GetCurrentStamina) 0.0)))