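; Blueprint function library of global shortcuts for reaching the project's core gameplay objects and setting UI focus.
; Getters return the first player's BP_MyPlayerCharacter and PC_MyPlayerController, plus BP_MyGameInstance, each cast from the generic engine accessor.
; SetMyFocus gives a button user focus for player 0's controller, then also applies keyboard focus and general focus.
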(fn GetMyPlayerCharacter
  (bind _asbp_my_player_character (Utilities|Casting|CastToBP_MyPlayerCharacter (Game|GetPlayerCharacter 0)))
  (return _asbp_my_player_character))

(fn GetMyPlayerController
  (bind _aspc_my_player_controller (Utilities|Casting|CastToPC_MyPlayerController (Game|GetPlayerController 0)))
  (return _aspc_my_player_controller))

(fn GetMyGameInstance
  (bind _asbp_my_game_instance (Utilities|Casting|CastToBP_MyGameInstance (Game|GetGameInstance)))
  (return _asbp_my_game_instance))

(fn SetMyFocus
  (params (Button :type Widget%20Object%20Reference))
  (Class|Widget|SetUserFocus Button (Game|GetPlayerController 0))
  (Widget|SetKeyboardFocus Button)
  (Widget|SetFocus Button))