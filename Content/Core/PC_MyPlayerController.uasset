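; Player controller that sets up input, camera pitch limits and the root UI widget, and handles pausing.
; On BeginPlay it adds the Enhanced Input mapping context, creates the UI root and opens the main menu for one GameState value.
; Common Input method changes toggle the cursor and apply the saved mouse or gamepad look sensitivity to the character.
; The pause action, allowed in the other GameState, toggles game pause and the pause menu.
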(event Custom|OnInputMethodChanged
  (params (bNewInputType :type ECommonInputType%20Enum :default "MouseAndKeyboard"))
  (bind _myplayercharacter (CallFunction|GetMyPlayerCharacter))
  (bind _mygameinstance (CallFunction|GetMyGameInstance))
  (bind _settingsdata (Variables|/Game/Core/BP_MyGameInstance.BP_MyGameInstance_C|GetSettingsData _mygameinstance))
  ;[0.15 0.15 0.15 0.5] Event Begin Play
  (switch Utilities|FlowControl|Switch|SwitchonECommonInputType bNewInputType
    (:MouseAndKeyboard
      (Variables|Default|SetbShowMouseCursor (Utilities|Enum|Equal(Enum) (Variables|Default|GetGameState) "NewEnumerator1"))
      (Utilities|IsValid _myplayercharacter
        (:Is%20Valid
          (Variables|/Game/Actors/MyPlayerCharacter/BP_MyPlayerCharacter.BP_MyPlayerCharacter_C|SetLookSensitivity _myplayercharacter (.mousesensitivity _settingsdata)))))
    (:Gamepad
      (Variables|Default|SetbShowMouseCursor false :!label _label)
      (Utilities|IsValid _myplayercharacter
        (:Is%20Valid
          (Variables|/Game/Actors/MyPlayerCharacter/BP_MyPlayerCharacter.BP_MyPlayerCharacter_C|SetLookSensitivity _myplayercharacter (.gamepadsensitivity _settingsdata)))))
    (:Touch
      (goto _label))
    (:Count
      (goto _label))))

(event Custom|TogglePause
  (if (not (Game|IsGamePaused))
    (Game|SetGamePaused true)
    (Default|OpenPauseMenu (Variables|Default|GetUIRoot))
    (else
      (Game|SetGamePaused false)
      (Variables|Default|SetbShowMouseCursor false)
      (Input|SetInputModeGameOnly self false)
      (Default|ClosePauseMenu (Variables|Default|GetUIRoot)))))

(event Input|EnhancedActionEvents|EnhancedInputActionIA_Pause
  (params (ActionValue :type Boolean) (ElapsedSeconds :type Float%20%28double-precision%29) (TriggeredSeconds :type Float%20%28double-precision%29) (InputAction :type Input%20Action%20Object%20Reference :default "/Game/Core/Input/IA_Pause.IA_Pause"))
  (:Started
    (if (Utilities|Enum|Equal(Enum) (Variables|Default|GetGameState) "NewEnumerator0")
      (CallFunction|TogglePause))))

(event EventBeginPlay
  (bind _returnvalue (PlayerController|LocalPlayerSubsystems|GetCommonInputSubsystem))
  (bind _playercameramanager (Variables|Default|GetPlayerCameraManager))
  ;[0.15 0.15 0.15 0.5] Event Begin Play
  (Input|AddMappingContext (PlayerController|LocalPlayerSubsystems|GetEnhancedInputLocalPlayerSubsystem self) "/Game/Core/Input/IMC_MyInputMap.IMC_MyInputMap" 0 "(bIgnoreAllPressedKeysUntilRelease=True,bForceImmediately=False,bNotifyUserSettings=False)")
  (Variables|/Script/Engine.PlayerCameraManager|SetViewPitchMin _playercameramanager -9e+01)
  (Variables|/Script/Engine.PlayerCameraManager|SetViewPitchMax _playercameramanager 65.0)
  (bind _returnvalue_2 (UserInterface|CreateWidget "/Game/Core/UI/WBP_UIRoot.WBP_UIRoot_C"))
  (bind _output_get (Variables|Default|SetUIRoot _returnvalue_2))
  (UserInterface|Viewport|AddtoViewport _output_get 0)
  (EventDispatchers|BindEventtoOnInputMethodChanged _returnvalue (delegate Custom|OnInputMethodChanged))
  (CallFunction|OnInputMethodChanged (Class|CommonInputSubsystem|GetDefaultInputType _returnvalue))
  (if (Utilities|Enum|Equal(Enum) (Variables|Default|GetGameState) "NewEnumerator1")
    (Default|OpenMainMenuWidget (Variables|Default|GetUIRoot))))

(fn ConstructionScript)